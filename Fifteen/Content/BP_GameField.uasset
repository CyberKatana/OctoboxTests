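; Game board for a 15-puzzle: spawns a 4x4 grid of numbered BP_Tile actors inside a box, leaving one empty slot.
; Start and Restart build the board from a plain shuffle, without a solvability check.
; Clicked tiles move when their array index is 1 or 4 from the free slot (row edges unchecked), swapping entries in Tiles.
; Each move checks tile Ids against array order and fires OnWin when sorted.
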(event `Restart`
  (bind _tiles (`self.Tiles`))
  (for _array_element _tiles
    (`/Engine/EditorBlueprintResources/StandardMacros.IsValid` _array_element
      (:`Is Valid`
        (remove `/Game/BP_Tile.OnTileClicked` _array_element (delegate `OnTileClicked`))
        (`self.K2_DestroyActor` _array_element))))
  (`KismetArrayLibrary.Array_Clear` _tiles)
  (`self.Start`))

(event `Start`
  (`self.SpawnTiles`)
  (for _array_element (`self.Tiles`)
    (`/Engine/EditorBlueprintResources/StandardMacros.IsValid` _array_element
      (:`Is Valid`
        (add `/Game/BP_Tile.OnTileClicked` _array_element (delegate `OnTileClicked`))))))

(event `OnTileClicked`
  (params (ClickedTile :type "/Game/BP_Tile Object Reference"))
  (switch `string` (`KismetStringLibrary.Conv_IntToString` (- (`self.FreeTileIndex`) (`KismetArrayLibrary.Array_Find` (`self.Tiles`) ClickedTile)))
    (:`-1`
      (set `self.Direction` "NewEnumerator0"))
    (:`1`
      (set `self.Direction` "NewEnumerator1"))
    (:`-4`
      (set `self.Direction` "NewEnumerator2"))
    (:`4`
      (set `self.Direction` "NewEnumerator3")))
  (`self.MoveTile` ClickedTile (`self.Direction`)))

(event `self.ReceiveBeginPlay`)

(fn `CheckTilesOrder`
  (for (_array_element _array_index) (`self.Tiles`)
    (if (< _array_index 15)
      (if (`KismetSystemLibrary.IsValid` _array_element)
        (if (!= (`/Game/BP_Tile.Id` _array_element) (+ _array_index 1))
          (return))
        (else
          (return)))))
  (`self.OnWin` self))

(fn `MoveTile`
  (params (Tile :type "/Game/BP_Tile Object Reference") (MoveDirection :type "/Game/E_MoveDirection Enum" :default "NewEnumerator0"))
  (locals (CachedIndex_Local :type Integer) (NewWorldPosition_Local :type "Vector Structure") (Step_Local :type "Vector Structure"))
  (bind _tiles (`self.Tiles`))
  (bind (_tileoffset_x _tileoffset_y) (`KismetMathLibrary.BreakVector` (`self.TileOffset`)))
  (bind _returnvalue (`KismetArrayLibrary.Array_Find` _tiles Tile))
  (switch `/Game/E_MoveDirection` MoveDirection
    (:`NewEnumerator0`
      (set `local.Step_Local` (`KismetMathLibrary.MakeVector` 0.0 (* _tileoffset_y -1.0))))
    (:`NewEnumerator1`
      (set `local.Step_Local` (`KismetMathLibrary.MakeVector` 0.0 _tileoffset_y)))
    (:`NewEnumerator2`
      (set `local.Step_Local` (`KismetMathLibrary.MakeVector` _tileoffset_x)))
    (:`NewEnumerator3`
      (set `local.Step_Local` (`KismetMathLibrary.MakeVector` (* _tileoffset_x -1.0)))))
  (`self.K2_SetActorLocation` Tile (+ (`local.Step_Local`) (`self.K2_GetActorLocation` Tile)) false true)
  (set `local.CachedIndex_Local` _returnvalue)
  (`KismetArrayLibrary.Array_Swap` _tiles _returnvalue (`self.FreeTileIndex`))
  (set `self.FreeTileIndex` (`local.CachedIndex_Local`))
  (`self.CheckTilesOrder`))

(fn `SpawnTiles`
  (locals (Slots :type "Array of Integer"))
  (bind (_worldpostionoffirsttile_x _worldpostionoffirsttile_y) (`KismetMathLibrary.BreakVector` (`self.WorldPostionOfFirstTile`)))
  (bind (_tileoffset_x _tileoffset_y) (`KismetMathLibrary.BreakVector` (`self.TileOffset`)))
  (bind (_tileoffset_x_2 _tileoffset_y_2) (`KismetMathLibrary.BreakVector` (`self.TileOffset`)))
  (bind (_returnvalue_x _returnvalue_y) (`KismetMathLibrary.BreakVector` (`SceneComponent.K2_GetComponentLocation` (`self.Box`))))
  (bind (_boxextent_x _boxextent_y) (`KismetMathLibrary.BreakVector` (`BoxComponent.BoxExtent` (`self.Box`))))
  (`KismetArrayLibrary.Array_Clear` (`local.Slots`))
  (for _index (range 1 16)
    (`KismetArrayLibrary.Array_Add` (`local.Slots`) _index))
  (`KismetArrayLibrary.Array_Shuffle` (`local.Slots`))
  (set `self.TileOffset` (`KismetMathLibrary.MakeVector` (/ _boxextent_x 2.0) (/ _boxextent_y 2.0)))
  (set `self.WorldPostionOfFirstTile` (`KismetMathLibrary.MakeVector` (- (+ _boxextent_x _returnvalue_x) (/ _tileoffset_x_2 2.0)) (+ (- _returnvalue_y _boxextent_y) (/ _tileoffset_y_2 2.0))))
  (for _index_2 (range 4)
    (for _index_3 (range 4)
      (bind _returnvalue (+ _index_3 (* _index_2 4)))
      (if (< (+ _returnvalue 1) 16)
        (bind _returnvalue_2 (`|SpawnActorFromClass` "/Game/BP_Tile.BP_Tile_C" (`KismetMathLibrary.MakeTransform` (`KismetMathLibrary.MakeVector` (- _worldpostionoffirsttile_x (* _tileoffset_x (`KismetMathLibrary.Conv_IntToDouble` _index_2))) (+ _worldpostionoffirsttile_y (* _tileoffset_y (`KismetMathLibrary.Conv_IntToDouble` _index_3))))) "Undefined" "OverrideRootScale" null (`|GetArrayItem` (`local.Slots`) _returnvalue) null))
        (`KismetArrayLibrary.Array_Add` (`self.Tiles`) _returnvalue_2)
        (else
          (bind _returnvalue_3 (`KismetArrayLibrary.Array_Add` (`self.Tiles`)))
          (set `self.FreeTileIndex` _returnvalue_3)
          (return))))))

(fn `UserConstructionScript`)