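; Player controller that owns the in-game menu UI and switches between menu and click-driven play.
; On BeginPlay it creates W_InGameUI with Game-and-UI input and binds its Start, Resume and Restart events.
; Those buttons hide the UI and re-enable click events, with Start and Restart also calling BP_GameMode.
; The Menu input and OnWin show their respective widget-switcher pages and disable click events.
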(event `self.ReceiveBeginPlay`
  (bind _gameui (`self.GameUI`))
  (set `self.bEnableClickEvents` false)
  (bind _returnvalue (`|CreateWidget` "/Game/W_InGameUI.W_InGameUI_C" self))
  (set `self.GameUI` _returnvalue)
  (`UserWidget.AddToViewport` (`self.GameUI`) 0)
  (`WidgetBlueprintLibrary.SetInputMode_GameAndUIEx` self (`self.GameUI`) "DoNotLock" false)
  (add `/Game/W_InGameUI.OnStartClicked` _gameui (delegate `OnStartClicked`))
  (add `/Game/W_InGameUI.OnResumeClicked` _gameui (delegate `OnResumeClicked`))
  (add `/Game/W_InGameUI.OnClickedRestart` _gameui (delegate `OnClickedRestart_Event_0`)))

(event `OnClickedRestart_Event_0`
  (bind _asbp_game_mode (cast `/Game/BP_GameMode` (`GameplayStatics.GetGameMode`)))
  (`/Game/BP_GameMode.Restart` _asbp_game_mode)
  (set `self.bEnableClickEvents` true)
  (`Widget.SetVisibility` (`self.GameUI`) "Hidden"))

(event `InputAction|Menu`
  (params (Key :type "Key Structure"))
  (bind _gameui (`self.GameUI`))
  (:`Pressed`
    (`Widget.SetVisibility` _gameui "Visible")
    (`WidgetSwitcher.SetActiveWidgetIndex` (`/Game/W_InGameUI.WidgetSwitcher_0` _gameui) 1)
    (set `self.bEnableClickEvents` false)))

(event `OnResumeClicked`
  (set `self.bEnableClickEvents` true)
  (`Widget.SetVisibility` (`self.GameUI`) "Hidden"))

(event `OnWin`
  (bind _gameui (`self.GameUI`))
  (`Widget.SetVisibility` _gameui "Visible")
  (`WidgetSwitcher.SetActiveWidgetIndex` (`/Game/W_InGameUI.WidgetSwitcher_0` _gameui) 2)
  (set `self.bEnableClickEvents` false))

(event `OnStartClicked`
  (set `self.bEnableClickEvents` true)
  (`Widget.SetVisibility` (`self.GameUI`) "Hidden")
  (bind _asbp_game_mode (cast `/Game/BP_GameMode` (`GameplayStatics.GetGameMode`)))
  (`/Game/BP_GameMode.Start` _asbp_game_mode))

(fn `UserConstructionScript`)