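; Grid playfield actor that runs a Snake game, spawning border walls, the snake and apples as BP_MapObject actors in a flat cell array.
; Tick drives timed turns that read the player controller's direction and wrap at map edges.
; Moves teleport the tail to the new head cell instead of shifting every part.
; Apples become the new head and shorten turn time; hitting the snake stops ticking and calls Loose on the controller.
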(event `self.ReceiveBeginPlay`
  (bind _asbp_player_controller (cast `/Game/BP_PlayerController` (`GameplayStatics.GetPlayerController` 0)))
  (set `self.PlayerController` _asbp_player_controller)
  (`self.SpawnWalls`))

(event `Restart`
  (bind _mapobject (`self.MapObject`))
  (`KismetArrayLibrary.Array_RemoveItem` _mapobject)
  (for _array_element _mapobject
    (`self.K2_DestroyActor` _array_element))
  (`self.Start`))

(event `Start`
  (set `self.TurnTime` 0.6)
  (`KismetArrayLibrary.Array_Clear` (`self.SnakeParts`))
  (`KismetArrayLibrary.Array_Resize` (`self.MapObject`) (* (`self.MapSizeX`) (`self.MapSizeY`)))
  (bind _returnvalue (`|SpawnActorFromClass` "/Game/BP_MapObject.BP_MapObject_C" (`KismetMathLibrary.MakeTransform` (`self.FirstCellLocation`)) "Undefined" "OverrideRootScale" null "NewEnumerator0" null))
  (`KismetArrayLibrary.Array_Set` (`self.MapObject`) 0 _returnvalue)
  (`KismetArrayLibrary.Array_Insert` (`self.SnakeParts`) _returnvalue)
  (`self.SpawnApple`)
  (`self.SetActorTickEnabled` true))

(event `self.ReceiveTick`
  (params (DeltaSeconds :type "Float (single-precision)"))
  (bind _output_get (set `self.TurnTimeCounter` (+ DeltaSeconds (`self.TurnTimeCounter`))))
  (if (>= _output_get (`self.TurnTime`))
    (set `self.TurnTimeCounter` (- (`self.TurnTimeCounter`) (`self.TurnTime`)))
    (set `self.SnakeDirection` (`/Game/BP_PlayerController.MovementDirection` (`self.PlayerController`)))
    (`self.MoveSnake`)))

(fn `ConvertIndexToXY`
  (params (ArrayIndex :type Integer))
  (returns (X :type Integer) (Y :type Integer))
  (bind _mapsizex (`self.MapSizeX`))
  (return (mod ArrayIndex _mapsizex) (/ ArrayIndex _mapsizex)))

(fn `ConvertXYToIndex`
  (params (X :type Integer) (Y :type Integer))
  (returns (ArrayIndex :type Integer))
  (return (+ X (* Y (`self.MapSizeX`)))))

(fn `GetFreeCell`
  (returns (RandomCellIndex :type Integer))
  (locals (RandomCellIndex_Local :type Integer :default 0))
  (set `local.RandomCellIndex_Local` (`KismetMathLibrary.RandomIntegerInRange` 0 (`KismetArrayLibrary.Array_LastIndex` (`self.MapObject`))))
  (while (`KismetSystemLibrary.IsValid` (`|GetArrayItem` (`self.MapObject`) (`local.RandomCellIndex_Local`))) :!label _label
    (set `local.RandomCellIndex_Local` (`KismetMathLibrary.RandomIntegerInRange` 0 (`KismetArrayLibrary.Array_LastIndex` (`self.MapObject`))))
    (goto _label))
  (return (`local.RandomCellIndex_Local`)))

(fn `HandleCollision`
  (params (CollidedObject :type "/Game/BP_MapObject Object Reference"))
  (switch `/Game/E_MapObjectTypes` (`/Game/BP_MapObject.Type` CollidedObject)
    (:`NewEnumerator0`
      (`/Game/BP_PlayerController.Loose` (`self.PlayerController`))
      (`self.SetActorTickEnabled` false))
    (:`NewEnumerator1`
      (`/Game/BP_MapObject.ChangeType` CollidedObject "NewEnumerator0")
      (`KismetArrayLibrary.Array_Insert` (`self.SnakeParts`) CollidedObject)
      (`self.SpawnApple`)
      (set `self.TurnTime` (* (`self.TurnTime`) 0.9)))))

(fn `MoveSnake`
  (locals (X_Local :type Integer :default 0) (Y_Local :type Integer :default 0) (HeadX_Local :type Integer) (HeadY_Local :type Integer) (HeadIndex_Local :type Integer :default 0) (CachedIndex_local :type Integer :default 0))
  (bind _snakeparts (`self.SnakeParts`))
  (bind _mapobject (`self.MapObject`))
  (bind _snakeparts_2 (`self.SnakeParts`))
  (bind _mapobject_2 (`self.MapObject`))
  (bind _returnvalue (`KismetArrayLibrary.Array_LastIndex` _snakeparts_2))
  (bind _returnvalue_2 (+ (`local.HeadY_Local`) 1))
  (bind _returnvalue_3 (+ (`local.HeadY_Local`) -1))
  (bind _returnvalue_4 (+ (`local.HeadX_Local`) 1))
  (bind _returnvalue_5 (+ (`local.HeadX_Local`) -1))
  (bind (_returnvalue_x _returnvalue_y _returnvalue_z) (`KismetMathLibrary.BreakVector` (`self.K2_GetActorLocation` (`|GetArrayItem` (`self.MapObject`) (`local.HeadIndex_Local`)))))
  (bind _returnvalue_6 (`KismetArrayLibrary.Array_Find` _mapobject_2 (`|GetArrayItem` _snakeparts (`KismetArrayLibrary.Array_LastIndex` _snakeparts))))
  (bind _output (`|GetArrayItem` _mapobject_2 _returnvalue_6))
  (bind _output_get (set `local.HeadIndex_Local` (`KismetArrayLibrary.Array_Find` (`self.MapObject`) (`|GetArrayItem` (`self.SnakeParts`)))))
  (bind (_x _y) (`self.ConvertIndexToXY` _output_get))
  (set `local.HeadX_Local` _x)
  (set `local.HeadY_Local` _y)
  (set `local.X_Local` (`local.HeadX_Local`))
  (set `local.Y_Local` (`local.HeadY_Local`))
  (switch `/Game/E_MovementDirection` (`self.SnakeDirection`)
    (:`NewEnumerator0`
      (set `local.X_Local` (select `bool` (>= _returnvalue_5 0) :`false` (- (`self.MapSizeX`) 1) :`true` _returnvalue_5)))
    (:`NewEnumerator1`
      (set `local.Y_Local` (select `bool` (>= _returnvalue_3 0) :`false` (- (`self.MapSizeY`) 1) :`true` _returnvalue_3)))
    (:`NewEnumerator2`
      (set `local.X_Local` (select `bool` (<= _returnvalue_4 (- (`self.MapSizeX`) 1)) :`true` _returnvalue_4)))
    (:`NewEnumerator3`
      (set `local.Y_Local` (select `bool` (<= _returnvalue_2 (- (`self.MapSizeY`) 1)) :`true` _returnvalue_2))))
  (bind _arrayindex (`self.ConvertXYToIndex` (`local.X_Local`) (`local.Y_Local`)))
  (bind _output_2 (`|GetArrayItem` (`self.MapObject`) _arrayindex))
  (`/Engine/EditorBlueprintResources/StandardMacros.IsValid` _output_2
    (:`Is Valid`
      (`self.HandleCollision` _output_2))
    (:`Is Not Valid`
      (`self.K2_SetActorLocation` _output (`KismetMathLibrary.MakeVector` (+ (* (- (`local.HeadY_Local`) (`local.Y_Local`)) (`self.CellSizeY`)) _returnvalue_x) (- _returnvalue_y (* (- (`local.HeadX_Local`) (`local.X_Local`)) (`self.CellSizeX`))) _returnvalue_z) false true)
      (set `local.CachedIndex_local` _returnvalue_6)
      (`KismetArrayLibrary.Array_Set` _mapobject _arrayindex _output)
      (`KismetArrayLibrary.Array_Set` _mapobject (`local.CachedIndex_local`))
      (`KismetArrayLibrary.Array_Insert` _snakeparts_2 (`|GetArrayItem` _snakeparts_2 _returnvalue))
      (`KismetArrayLibrary.Array_Remove` _snakeparts_2 _returnvalue))))

(fn `SpawnApple`
  (bind (_firstcelllocation_x _firstcelllocation_y _firstcelllocation_z) (`KismetMathLibrary.BreakVector` (`self.FirstCellLocation`)))
  (bind _randomcellindex (`self.GetFreeCell`))
  (bind (_x _y) (`self.ConvertIndexToXY` _randomcellindex))
  (bind _returnvalue (`|SpawnActorFromClass` "/Game/BP_MapObject.BP_MapObject_C" (`KismetMathLibrary.MakeTransform` (`KismetMathLibrary.MakeVector` (- _firstcelllocation_x (* _y (`self.CellSizeY`))) (+ (* _x (`self.CellSizeX`)) _firstcelllocation_y) _firstcelllocation_z)) "Undefined" "OverrideRootScale" null "NewEnumerator1" null))
  (`KismetArrayLibrary.Array_Set` (`self.MapObject`) _randomcellindex _returnvalue))

(fn `SpawnWalls`
  (bind (_firstcelllocation_x _firstcelllocation_y _firstcelllocation_z) (`KismetMathLibrary.BreakVector` (`self.FirstCellLocation`)))
  (for _index (range (+ (+ (`self.MapSizeX`) 1) 1))
    (for _index_2 (range (+ (+ (`self.MapSizeY`) 1) 1))
      (bind _returnvalue (- _index 1))
      (bind _returnvalue_2 (- _index_2 1))
      (if (or (< _returnvalue 0) (== _returnvalue (`self.MapSizeX`)) (< _returnvalue_2 0) (== _returnvalue_2 (`self.MapSizeY`)))
        (`|SpawnActorFromClass` "/Game/BP_MapObject.BP_MapObject_C" (`KismetMathLibrary.MakeTransform` (`KismetMathLibrary.MakeVector` (+ (* (* _returnvalue_2 -1) (`self.CellSizeY`)) _firstcelllocation_x) (+ (* _returnvalue (`self.CellSizeX`)) _firstcelllocation_y) _firstcelllocation_z)) "Undefined" "OverrideRootScale" null "NewEnumerator2" null)))))

(fn `UserConstructionScript`
  (locals (OffsetX_Local :type "Float (double-precision)" :default 0.0) (OffsetY_Local :type "Float (double-precision)" :default 0.0))
  (bind (_returnvalue_x _returnvalue_y _returnvalue_z) (`KismetMathLibrary.BreakVector` (`self.K2_GetActorLocation`)))
  (bind _mapsizex (`self.MapSizeX`))
  (bind _cellsizex (`self.CellSizeX`))
  (bind _mapsizey (`self.MapSizeY`))
  (bind _cellsizey (`self.CellSizeY`))
  (set `local.OffsetX_Local` (`KismetMathLibrary.SelectFloat` (* (/ _mapsizex 2) _cellsizex) (* _cellsizex (/ (`KismetMathLibrary.Conv_IntToDouble` _mapsizex) 2.0)) (> (mod _mapsizex 2) 0)))
  (set `local.OffsetY_Local` (`KismetMathLibrary.SelectFloat` (* (/ _mapsizey 2) _cellsizey) (* _cellsizey (/ (`KismetMathLibrary.Conv_IntToDouble` _mapsizey) 2.0)) (> (mod _mapsizey 2) 0)))
  (set `self.FirstCellLocation` (`KismetMathLibrary.MakeVector` (+ (`local.OffsetY_Local`) _returnvalue_x) (- _returnvalue_y (`local.OffsetX_Local`)) _returnvalue_z)))