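; Player controller for a grid-style directional game that owns the current movement direction and the start and game-over UI flow.
; BeginPlay picks a random direction and shows W_InGameUI, whose Start and Restart events hide it and call BP_GameField.
; Direction inputs only allow perpendicular turns, preventing reversals.
; Loose switches the widget to its second page and restores UI-only input with the cursor.
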(event `self.ReceiveBeginPlay`
  (bind _gameui (`self.GameUI`))
  (set `self.MovementDirection` (cast `/Game/E_MovementDirection` (`KismetMathLibrary.Conv_IntToByte` (`KismetMathLibrary.RandomIntegerInRange` 0 3))))
  (set `self.bShowMouseCursor` true)
  (bind _returnvalue (`|CreateWidget` "/Game/W_InGameUI.W_InGameUI_C"))
  (set `self.GameUI` _returnvalue)
  (`UserWidget.AddToViewport` _gameui 0)
  (`WidgetBlueprintLibrary.SetInputMode_UIOnlyEx` self _gameui)
  (add `/Game/W_InGameUI.OnStartClicked` _gameui (delegate `OnStartClicked_Event_0`))
  (add `/Game/W_InGameUI.OnClickedRestart` (`self.GameUI`) (delegate `OnClickedRestart_Event_0`)))

(event `OnClickedRestart_Event_0`
  (set `self.bShowMouseCursor` false)
  (`Widget.SetVisibility` (`self.GameUI`) "Hidden")
  (bind _outactors (`GameplayStatics.GetAllActorsOfClass` "/Game/BP_GameField.BP_GameField_C"))
  (`/Game/BP_GameField.Restart` (`|GetArrayItem` _outactors))
  (`WidgetBlueprintLibrary.SetInputMode_GameOnly` self)
  (set `self.MovementDirection` (cast `/Game/E_MovementDirection` (`KismetMathLibrary.Conv_IntToByte` (`KismetMathLibrary.RandomIntegerInRange` 0 3)))))

(event `InputAction|Up`
  (params (Key :type "Key Structure"))
  (:`Pressed`
    (switch `/Game/E_MovementDirection` (`self.MovementDirection`)
      (:`NewEnumerator0`
        _)
      (:`NewEnumerator2`
        _))
    (set `self.MovementDirection` "NewEnumerator1")))

(event `OnStartClicked_Event_0`
  (set `self.bShowMouseCursor` false)
  (`Widget.SetVisibility` (`self.GameUI`) "Hidden")
  (bind _outactors (`GameplayStatics.GetAllActorsOfClass` "/Game/BP_GameField.BP_GameField_C"))
  (`/Game/BP_GameField.Start` (`|GetArrayItem` _outactors))
  (`WidgetBlueprintLibrary.SetInputMode_GameOnly` self))

(event `InputAction|Down`
  (params (Key :type "Key Structure"))
  (:`Pressed`
    (switch `/Game/E_MovementDirection` (`self.MovementDirection`)
      (:`NewEnumerator0`
        _)
      (:`NewEnumerator2`
        _))
    (set `self.MovementDirection` "NewEnumerator3")))

(event `InputAction|Left`
  (params (Key :type "Key Structure"))
  (:`Pressed`
    (switch `/Game/E_MovementDirection` (`self.MovementDirection`)
      (:`NewEnumerator1`
        _)
      (:`NewEnumerator3`
        _))
    (set `self.MovementDirection` "NewEnumerator0")))

(event `InputAction|Right`
  (params (Key :type "Key Structure"))
  (:`Pressed`
    (switch `/Game/E_MovementDirection` (`self.MovementDirection`)
      (:`NewEnumerator1`
        _)
      (:`NewEnumerator3`
        _))
    (set `self.MovementDirection` "NewEnumerator2")))

(event `Loose`
  (`WidgetSwitcher.SetActiveWidgetIndex` (`/Game/W_InGameUI.WidgetSwitcher_0` (`self.GameUI`)) 1)
  (`Widget.SetVisibility` (`self.GameUI`) "Visible")
  (set `self.bShowMouseCursor` true)
  (`WidgetBlueprintLibrary.SetInputMode_UIOnlyEx` self (`self.GameUI`)))

(fn `UserConstructionScript`)