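; Game mode that links game fields to the player controller and relays start and restart commands.
; On BeginPlay it binds to the OnWin dispatcher of every BP_GameField in the level, forwarding a win to OnWin on player 0's BP_PlayerController.
; Its Start and Restart events call the matching function on the first game field found.
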(event `self.ReceiveBeginPlay`
  (bind _outactors (`GameplayStatics.GetAllActorsOfClass` "/Game/BP_GameField.BP_GameField_C"))
  (for _array_element _outactors
    (add `/Game/BP_GameField.OnWin` _array_element (delegate `OnWin_Event_0`))))

(event `OnWin_Event_0`
  (params (GameField :type "/Game/BP_GameField Object Reference"))
  (bind _asbp_player_controller (cast `/Game/BP_PlayerController` (`GameplayStatics.GetPlayerController` 0)))
  (`/Game/BP_PlayerController.OnWin` _asbp_player_controller))

(event `Start`
  (bind _outactors (`GameplayStatics.GetAllActorsOfClass` "/Game/BP_GameField.BP_GameField_C"))
  (`/Game/BP_GameField.Start` (`|GetArrayItem` _outactors)))

(event `Restart`
  (bind _outactors (`GameplayStatics.GetAllActorsOfClass` "/Game/BP_GameField.BP_GameField_C"))
  (`/Game/BP_GameField.Restart` (`|GetArrayItem` _outactors)))

(fn `UserConstructionScript`)